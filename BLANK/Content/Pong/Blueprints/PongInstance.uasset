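; PongInstance keeps the left and right scores for a Pong game.
; Its single AddScore event adds the given points to one side, chosen by a boolean input.
; It then prints both totals as a combined string through PrintString.
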(event Custom|AddScore
  (params (Points :type Integer) (Left%20Score :type Boolean))
  (if Left%20Score
    (Variables|Default|SetLeft%20Score (+ (Variables|Default|GetLeft%20Score) Points))
    (else
      (Variables|Default|SetRight%20Score (+ Points (Variables|Default|GetRight%20Score)))))
  (Development|PrintString (Utilities|String|Append "Left  Score: " (Utilities|String|ToString(Integer) (Variables|Default|GetLeft%20Score)) "Right Score: " (Utilities|String|ToString(Integer) (Variables|Default|GetRight%20Score)))))